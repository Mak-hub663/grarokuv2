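; Moving platform that starts travelling toward a configurable relative position when the player's Ziomo1BP character enters its box trigger.
; The construction script builds the InterpToMovement path from two relative control points, the origin and MoveToPos.
; BeginPlay caches the player character, and its first overlap with the box passes a DoOnce, waits the configurable Opoznienieplatformyup delay, then activates the movement component.
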(event `self.ReceiveBeginPlay`
  (bind _asziomo_1bp (cast `/Game/Ziomo1BP` (`GameplayStatics.GetPlayerCharacter` 0)))
  (set `self.As Ziomo 1BP` _asziomo_1bp))

(event `self.Box.OnComponentBeginOverlap`
  (params (OverlappedComponent :type "PrimitiveComponent Object Reference") (OtherActor :type "Actor Object Reference") (OtherComp :type "PrimitiveComponent Object Reference") (OtherBodyIndex :type Integer) (bFromSweep :type Boolean) (SweepResult :type "HitResult Structure (by ref)"))
  (if (== OtherActor (`self.As Ziomo 1BP`))
    (`/Engine/EditorBlueprintResources/StandardMacros.DoOnce` false
      (:`Completed`
        (`KismetSystemLibrary.Delay` (`KismetMathLibrary.Conv_IntToDouble` (`self.opoznienieplatformyup`)))
        (`ActorComponent.Activate` (`self.InterpToMovement`) false)))))

(fn `UserConstructionScript`
  (`InterpToMovementComponent.AddControlPointPosition` (`self.InterpToMovement`) (0.0 0.0 0.0) true)
  (`InterpToMovementComponent.AddControlPointPosition` (`self.InterpToMovement`) (`self.moveToPos`) true))